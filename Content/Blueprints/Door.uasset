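; Door Blueprint that swings open once enough items have been collected.
; CollectItem increments a counter and, when it reaches the maximum, fires OpenDoor a single time through a DoOnce.
; OpenDoor plays a timeline that lerps the yaw of both LeftDoor meshes from closed to a right angle.
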(event `OpenDoor`
  (bind (_direction _door_rotation) (`Timeline|Open Door Anim`)
    (:`Update`
      (`SceneComponent.K2_SetRelativeRotation` (`self.leftDoor`) (`KismetMathLibrary.MakeRotator` 0.0 0.0 (`KismetMathLibrary.Lerp` 0.0 90.0 _door_rotation)) false false)
      (`SceneComponent.K2_SetRelativeRotation` (`self.leftDoor1`) (`KismetMathLibrary.MakeRotator` 0.0 0.0 (`KismetMathLibrary.Lerp` 0.0 90.0 _door_rotation)) false false))))

(event `Collect Item`
  (`/Engine/EditorBlueprintResources/StandardMacros.IncrementInt` (`self.currentItemsCollected`)
    (:`  `
      (if (>= (`self.currentItemsCollected`) (`self.maxItemsCollectable`))
        (`/Engine/EditorBlueprintResources/StandardMacros.DoOnce` false
          (:`Completed`
            (`self.OpenDoor`)))))))

(fn `UserConstructionScript`)