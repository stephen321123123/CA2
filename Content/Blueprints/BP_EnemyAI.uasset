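; BP_EnemyAI is an enemy character that chases the player and attacks on reaching them.
; PawnSensing sets IsSeeingPlayer and starts an AIMoveTo toward the player, while Tick stops movement whenever that flag is false.
; A successful move plays a pistol-fire montage, with CanAttack and a montage-length Delay intended as a cooldown.
; Damage is separate from the montage: a Box overlap damages any overlapping actor.
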(event `self.ReceiveTick`
  (params (DeltaSeconds :type "Float (single-precision)"))
  ; Enemy Stops Following
  (if (not (`self.isSeeingPlayer`))
    (`Controller.StopMovement` (`self.GetController`))))

(event `FollowPlayer`
  ; Functionality of Enemy Movement
  (set `self.canAttack?` true)
  (if (`self.isSeeingPlayer`)
    (`|AIMoveTo` self (0.0 0.0 0.0) (`GameplayStatics.GetPlayerCharacter` 0) 50.0
      (:`OnSuccess`
        (if (`self.canAttack?`)
          (set `self.canAttack?` false)
          (bind _returnvalue (`self.PlayAnimMontage` "/Game/Characters/Mannequins/Anims/Pistol/MM_Pistol_Fire_Montage.MM_Pistol_Fire_Montage" 0.5))
          (`KismetSystemLibrary.Delay` _returnvalue)
          (set `self.canAttack?` true))))
    (else
      (set `self.isSeeingPlayer` false))))

(event `self.PawnSensing.OnSeePawn`
  (params (Pawn :type "Pawn Object Reference"))
  ; Enemy Follows Player
  (set `self.isSeeingPlayer` true)
  (`self.FollowPlayer`))

(event `self. Box.OnComponentBeginOverlap`
  (params (OverlappedComponent :type "PrimitiveComponent Object Reference") (OtherActor :type "Actor Object Reference") (OtherComp :type "PrimitiveComponent Object Reference") (OtherBodyIndex :type Integer) (bFromSweep :type Boolean) (SweepResult :type "HitResult Structure (by ref)"))
  (`GameplayStatics.ApplyDamage` OtherActor 25.0))

(fn `UserConstructionScript`)